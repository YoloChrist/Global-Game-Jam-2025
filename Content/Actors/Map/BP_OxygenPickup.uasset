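; BP_OxygenPickup is a map actor that refills the player's oxygen when collected.
; On BeginPlay it caches the BP_GameInstance.
; When a BP_ThirdPersonCharacter overlaps it, it adds its Oxygen value divided by the game instance's Difficulty to PlayerOxygen, then destroys itself.
; The addition is applied without a clamp.
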(event Collision|EventActorBeginOverlap
  (params (OtherActor :type Actor%20Object%20Reference))
  (bind _asbp_third_person_character (Utilities|Casting|CastToBP_ThirdPersonCharacter OtherActor))
  (Variables|/Game/ThirdPerson/Blueprints/BP_ThirdPersonCharacter.BP_ThirdPersonCharacter_C|SetplayerOxygen _asbp_third_person_character (+ (/ (Variables|Default|GetOxygen) (Variables|/Game/Actors/BP_GameInstance.BP_GameInstance_C|GetDifficulty (stale EventBeginPlay _asbp_game_instance))) (Variables|/Game/ThirdPerson/Blueprints/BP_ThirdPersonCharacter.BP_ThirdPersonCharacter_C|GetplayerOxygen _asbp_third_person_character)))
  (Actor|DestroyActor))

(event EventBeginPlay
  (bind _asbp_game_instance (Utilities|Casting|CastToBP_GameInstance (Game|GetGameInstance))))

(fn ConstructionScript)